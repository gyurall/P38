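; P-38 airplane Actor that spins its two propellers and flies in a straight line.
; Each Tick rolls the Right and Left propeller components locally by RotationSpeed scaled by delta time, through a shared RotationPropeller function.
; MoveForward then offsets the actor along world X at a fixed, frame-rate-independent speed, regardless of its facing.
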(event `self.ReceiveTick`
  (params (DeltaSeconds :type "Float (single-precision)"))
  ;[1 1 1] 오른쪽 회전
  (`self.Rotation Propeller` (`self.Right`))
  ;[1 1 1] 왼쪽 회전
  (`self.Rotation Propeller` (`self.Left`))
  ;[1 1 1] 비행기 이동
  (`self.MoveForward`))

(fn `MoveForward`
  (`self.K2_AddActorWorldOffset` (`KismetMathLibrary.MakeVector` (* 100.0 (`GameplayStatics.GetWorldDeltaSeconds`)))))

(fn `Rotation Propeller`
  (params (self2 :type "SceneComponent Object Reference"))
  (`SceneComponent.K2_AddLocalRotation` self2 (`KismetMathLibrary.MakeRotator` (* (`GameplayStatics.GetWorldDeltaSeconds`) (`self.RotationSpeed`))) false false))

(fn `UserConstructionScript`)